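; CaveEntrance_BP is a level transition trigger that saves the player's progress and moves them to the next level.
; When the FirstPersonCharacter overlaps its trigger, it writes inventory, health and the NextLevel name into a MySaveOptions save object in the "save" slot.
; It then shows a LoadScreenUI widget and opens the NextLevel map by name after a short delay.
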(event OnComponentBeginOverlap(Trigger)
  (params (OverlappedComponent :type Primitive%20Component%20Object%20Reference) (OtherActor :type Actor%20Object%20Reference) (OtherComp :type Primitive%20Component%20Object%20Reference) (OtherBodyIndex :type Integer) (bFromSweep :type Boolean) (SweepResult :type Hit%20Result%20Structure%20%28by%20ref%29))
  (bind _asfirst_person_character (Utilities|Casting|CastToFirstPersonCharacter OtherActor))
  (bind _returnvalue (SaveGame|CreateSaveGameObject "/Game/MyBlueprints/MySaveOptions.MySaveOptions_C"))
  (Variables|/Game/MyBlueprints/MySaveOptions.MySaveOptions_C|SetInventory _returnvalue (Variables|/Game/UMG/Inventory/InventoryMenu.InventoryMenu_C|GetInventory (Variables|/Game/FirstPersonBP/Blueprints/FirstPersonCharacter.FirstPersonCharacter_C|GetInventoryUI _asfirst_person_character)))
  (Variables|/Game/MyBlueprints/MySaveOptions.MySaveOptions_C|SetHealth _returnvalue (Variables|/Game/FirstPersonBP/Blueprints/FirstPersonCharacter.FirstPersonCharacter_C|GetHealth _asfirst_person_character))
  (Variables|/Game/MyBlueprints/MySaveOptions.MySaveOptions_C|SetLevelName _returnvalue (Variables|Default|GetNextLevel))
  (SaveGame|SaveGametoSlot _returnvalue "save")
  (bind _returnvalue_2 (UserInterface|CreateWidget "/Game/UMG/LoadScreenUI.LoadScreenUI_C"))
  (UserInterface|Viewport|AddtoViewport _returnvalue_2 0)
  (Utilities|FlowControl|Delay 1.0)
  (Game|OpenLevel(byName) (Utilities|String|StringToName (Variables|Default|GetNextLevel))))

(fn ConstructionScript)