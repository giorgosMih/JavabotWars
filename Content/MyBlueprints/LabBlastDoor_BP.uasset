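; Lab blast door that opens as the player enters the rear trigger and closes once the front trigger is reached.
; A timeline offsets the door from its initial relative location, playing forward to open and in reverse to close.
; Closing also switches a blocking volume to an invisible wall profile.
; When each movement finishes, spent triggers are destroyed, along with the blocking volume after closing, making the sequence one-time.
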(event OnComponentBeginOverlap(rear_trigger)
  (params (OverlappedComponent :type Primitive%20Component%20Object%20Reference) (OtherActor :type Actor%20Object%20Reference) (OtherComp :type Primitive%20Component%20Object%20Reference) (OtherBodyIndex :type Integer) (bFromSweep :type Boolean) (SweepResult :type Hit%20Result%20Structure%20%28by%20ref%29))
  (bind _rear_trigger (Variables|Default|Getrear_trigger))
  ;[0.315 1 0.4792] Open Blast Door
  (Utilities|Casting|CastToFirstPersonCharacter OtherActor)
  (bind _movement (Timeline|MoveBlastDoor Play)
    (:Update
      (Transformation|SetRelativeLocation (Variables|Default|Getdoor) (+ _movement (Variables|Default|GetBlastDoor_location)) false false))
    (:Finished
      ;[1 1 1] Destroy Triggers
      (if (Variables|Default|GetBlastDoorClosed)
        ;;[1 0.9196 0.1415] Destroy Closing Trigger (and Opening Trigger if not destroyed)
        (Components|DestroyComponent (Variables|Default|Getfront_trigger))
        (Components|DestroyComponent (Variables|Default|Getblocking_volume))
        (Utilities|IsValid _rear_trigger
          (:Is%20Valid
            _)))
      ;;;[0.257 0.2402 1] Destroy Opening Trigger
      (Components|DestroyComponent _rear_trigger))))

(event OnComponentBeginOverlap(front_trigger)
  (params (OverlappedComponent :type Primitive%20Component%20Object%20Reference) (OtherActor :type Actor%20Object%20Reference) (OtherComp :type Primitive%20Component%20Object%20Reference) (OtherBodyIndex :type Integer) (bFromSweep :type Boolean) (SweepResult :type Hit%20Result%20Structure%20%28by%20ref%29))
  (bind _rear_trigger (Variables|Default|Getrear_trigger))
  ;[1 0.2643 0.1946] Close Blast Door
  (Utilities|Casting|CastToFirstPersonCharacter OtherActor)
  (Collision|SetCollisionProfileName (Variables|Default|Getblocking_volume) "InvisibleWall" :!class /Script/Engine.PrimitiveComponent)
  (Variables|Default|SetBlastDoorClosed true)
  ;[0.315 1 0.4792] Open Blast Door
  (bind _movement (Timeline|MoveBlastDoor Reverse)
    (:Update
      (Transformation|SetRelativeLocation (Variables|Default|Getdoor) (+ _movement (Variables|Default|GetBlastDoor_location)) false false))
    (:Finished
      ;[1 1 1] Destroy Triggers
      (if (Variables|Default|GetBlastDoorClosed)
        ;;[1 0.9196 0.1415] Destroy Closing Trigger (and Opening Trigger if not destroyed)
        (Components|DestroyComponent (Variables|Default|Getfront_trigger))
        (Components|DestroyComponent (Variables|Default|Getblocking_volume))
        (Utilities|IsValid _rear_trigger
          (:Is%20Valid
            _)))
      ;;;[0.257 0.2402 1] Destroy Opening Trigger
      (Components|DestroyComponent _rear_trigger))))

(event EventBeginPlay
  ;[1 1 1] Begin Play
  (Variables|Default|SetBlastDoor_location (Variables|/Script/Engine.SceneComponent|GetRelativeLocation (Variables|Default|Getdoor))))

(fn ConstructionScript)