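; Painting actor that displays a configurable PaintingMaterial on the first material slot of its Painting component.
; The construction script rescales that component from the actor's relative scale, multiplying X by actor Y and Y by the actor's Z-to-Y ratio.
; It also applies the material there, and BeginPlay applies it again when play starts.
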(event EventBeginPlay
  (Rendering|Material|SetMaterial (Variables|Default|GetPainting) 0 (Variables|Default|GetPaintingMaterial)))

(fn ConstructionScript
  (bind _returnvalue (Class|Actor|GetActorRelativeScale3D))
  (bind _painting (Variables|Default|GetPainting))
  (bind (_x _y _z) (Math|Vector|BreakVector _returnvalue))
  (bind _relativescale3d (Variables|/Script/Engine.SceneComponent|GetRelativeScale3D _painting))
  (bind (_x_2 _y_2 _z_2) (Math|Vector|BreakVector _relativescale3d))
  (Transformation|SetRelativeScale3D _painting (Math|Vector|MakeVector (* _y _x_2) (/ (* _z _y_2) _y) _z_2))
  (Rendering|Material|SetMaterial (Variables|Default|GetPainting) 0 (Variables|Default|GetPaintingMaterial)))