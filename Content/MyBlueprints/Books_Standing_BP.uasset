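; Procedural prop Blueprint that builds a row of standing books with random cover colors.
; The construction script adds NumOfBooks copies of the Book mesh, each offset by Distance along negative X from the previous one, starting at RootBook.
; Every book, including RootBook and TiltedBook, gets a dynamic M_BasicBook material with a random Color, re-rolled on each construction run.
; TiltedBook is destroyed when HasTilted is off.
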(event EventBeginPlay)

(event Collision|EventActorBeginOverlap
  (params (OtherActor :type Actor%20Object%20Reference)))

(event EventTick
  (params (DeltaSeconds :type Float%20%28single-precision%29)))

(fn ConstructionScript
  (bind _books (Variables|Default|GetBooks))
  (bind _books_2 (Variables|Default|GetBooks))
  (bind _rootbook (Variables|Default|GetRootBook))
  (bind _returnvalue (Transformation|GetRelativeTransform _rootbook))
  (bind (_location _rotation _scale) (Math|Transform|BreakTransform _returnvalue))
  (bind (_x _y _z) (Math|Vector|BreakVector _location))
  (for _index (range 0 (- (Variables|Default|GetNumOfBooks) 1))
    (if (== _index 0)
      (bind _returnvalue_2 (AddComponent|AddStaticMeshComponent false (Math|Transform|MakeTransform (Math|Vector|MakeVector (- _x (Variables|Default|GetDistance)) _y _z) _rotation _scale)))
      (Components|StaticMesh|SetStaticMesh _returnvalue_2 "/Game/MyMeshes/Book.Book")
      (Utilities|Array|Add _books _returnvalue_2)
      (else
        (bind _returnvalue_3 (AddComponent|AddStaticMeshComponent false (Math|Transform|MakeTransform (Math|Vector|MakeVector (- (.X (Math|Vector|BreakVector (.Location (Math|Transform|BreakTransform (Transformation|GetRelativeTransform (Utilities|Array|Get(acopy) (Variables|Default|GetBooks) (- _index 1))))))) (Variables|Default|GetDistance)) (.Y (Math|Vector|BreakVector (.Location (Math|Transform|BreakTransform (Transformation|GetRelativeTransform (Utilities|Array|Get(acopy) (Variables|Default|GetBooks) (- _index 1))))))) (.Z (Math|Vector|BreakVector (.Location (Math|Transform|BreakTransform (Transformation|GetRelativeTransform (Utilities|Array|Get(acopy) (Variables|Default|GetBooks) (- _index 1)))))))) (.Rotation (Math|Transform|BreakTransform (Transformation|GetRelativeTransform (Utilities|Array|Get(acopy) (Variables|Default|GetBooks) (- _index 1))))) (.Scale (Math|Transform|BreakTransform (Transformation|GetRelativeTransform (Utilities|Array|Get(acopy) (Variables|Default|GetBooks) (- _index 1))))))))
        (Components|StaticMesh|SetStaticMesh _returnvalue_3 "/Game/MyMeshes/Book.Book")
        (Utilities|Array|Add _books _returnvalue_3))))
  (Utilities|Array|Add _books_2 (Variables|Default|GetRootBook))
  (Utilities|Array|Add _books_2 (Variables|Default|GetTiltedBook))
  (for _array_element _books_2
    (bind _returnvalue_4 (Rendering|Material|CreateDynamicMaterialInstance _array_element 0 "/Game/MyMaterials/M_BasicBook.M_BasicBook" :!class /Script/Engine.PrimitiveComponent))
    (Rendering|Material|SetVectorParameterValue _returnvalue_4 "Color" (Utilities|Struct|MakeLinearColor (Math|Random|RandomFloatinRange 0.0 1.0) (Math|Random|RandomFloatinRange 0.0 1.0) (Math|Random|RandomFloatinRange 0.0 1.0) 1.0) :!class /Script/Engine.MaterialInstanceDynamic))
  (Utilities|Array|Clear (Variables|Default|GetBooks))
  (if (not (Variables|Default|GetHasTilted))
    (Components|DestroyComponent (Variables|Default|GetTiltedBook))))